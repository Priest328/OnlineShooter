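; BP_SCharacter is a character Blueprint that starts play armed with a grenade launcher and a crosshair on screen.
; On BeginPlay it spawns BP_GrenadeLauncher, stores it as CurrentWeapon, snaps it to the mesh's hand_WeaponrSocket and adds the WBP_Crosshair widget to the viewport.
; Left mouse button press calls Fire on CurrentWeapon through a direct key event.
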(event `Key|LeftMouseButton`
  (params (Key :type "Key Structure"))
  (:`Pressed`
    (`OSWeapon.Fire` (`self.Current weapon`))))

(event `self.ReceiveBeginPlay`
  (bind _returnvalue (`|SpawnActorFromClass` "/Game/BP_GrenadeLauncher.BP_GrenadeLauncher_C" (`KismetMathLibrary.MakeTransform` (0.0 0.0 0.0)) "AlwaysSpawn" "MultiplyWithRoot" self null))
  (set `self.Current weapon` _returnvalue)
  (`self.K2_AttachToComponent` _returnvalue (`self.Mesh`) "hand_WeaponrSocket" "SnapToTarget" "SnapToTarget" "SnapToTarget" true)
  (bind _returnvalue_2 (`|CreateWidget` "/Game/UI/WBP_Crosshair.WBP_Crosshair_C"))
  (`UserWidget.AddToViewport` _returnvalue_2 0))

(fn `UserConstructionScript`)